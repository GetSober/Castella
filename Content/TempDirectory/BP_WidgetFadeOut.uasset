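; BP_WidgetFadeOut is an actor that fades the screen with a black overlay and then loads another level.
; Its Action event adds a WBP_Screen widget to the viewport and plays a timeline whose length is set to FadeTime.
; Each update samples FadeCurve at the normalized playback position to drive the overlay's alpha.
; When the timeline finishes, it opens NextLevel by object reference.
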(event `self.ReceiveBeginPlay`
  (`parent.ReceiveBeginPlay`))

(event `/Game/Blueprints/BPI_Queue.Action`
  (bind _update_widge (`self.Update Widge`))
  (bind _returnvalue (`|CreateWidget` "/Game/TempDirectory/WBP_Screen.WBP_Screen_C" (`GameplayStatics.GetPlayerController` 0)))
  (`UserWidget.AddToViewport` _returnvalue 0)
  (`TimelineComponent.SetTimelineLength` _update_widge (`self.FadeTime`))
  (`Timeline|Update Widge`
    (:`Update`
      (`/Game/TempDirectory/WBP_Screen.UpdateScreen` _returnvalue (make `LinearColor` 0.0 0.0 0.0 (`CurveFloat.GetFloatValue` (`self.FadeCurve`) (/ (`TimelineComponent.GetPlaybackPosition` _update_widge) (`TimelineComponent.GetTimelineLength` _update_widge))))))
    (:`Finished`
      (`GameplayStatics.OpenLevelBySoftObjectPtr` (`self.NextLevel`)))))

(fn `UserConstructionScript`
  (`parent.UserConstructionScript`))