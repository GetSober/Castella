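; Actor that plays a media video in a WBP_Screen viewport widget with faded opacity.
; BeginPlay opens the media source; Action creates the widget, starts playback and runs the FadeIn timeline.
; Tick starts FadeOut once remaining playback reaches FadeOutTime, then ends and hides the widget.
; Both timelines drive Opacity in MTPC_Media through FadeCurve, reversed for fade-out, and both take their length from FadeInTime.
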(event `self.ReceiveBeginPlay`
  (`parent.ReceiveBeginPlay`)
  (`MediaPlayer.OpenSource` (`self.Media Player`) (`self.MediaSource`)))

(event `self.ReceiveTick`
  (params (DeltaSeconds :type "Float (single-precision)"))
  (bind _media_player (`self.Media Player`))
  (bind _widget (`self.Widget`))
  (bind _fadeout (`self.FadeOut`))
  (bind (_returnvalue_days _returnvalue_hours _returnvalue_minutes _returnvalue_seconds) (`KismetMathLibrary.BreakTimespan` (`MediaPlayer.GetDuration` _media_player)))
  (bind (_returnvalue_days_2 _returnvalue_hours_2 _returnvalue_minutes_2 _returnvalue_seconds_2) (`KismetMathLibrary.BreakTimespan` (`MediaPlayer.GetTime` _media_player)))
  (`parent.ReceiveTick` DeltaSeconds)
  (if (`MediaPlayer.IsPlaying` _media_player)
    (if (<= (- _returnvalue_seconds _returnvalue_seconds_2) (`self.FadeOutTime`))
      (`TimelineComponent.SetTimelineLength` _fadeout (`self.FadeInTime`))
      (`Timeline|FadeOut`
        (:`Update`
          (`KismetMaterialLibrary.SetScalarParameterValue` "/Game/TempDirectory/MTPC_Media.MTPC_Media" "Opacity" (`CurveFloat.GetFloatValue` (`self.FadeCurve`) (- 1.0 (/ (`TimelineComponent.GetPlaybackPosition` _fadeout) (`TimelineComponent.GetTimelineLength` _fadeout))))))
        (:`Finished`
          (`/Game/TempDirectory/WBP_Screen.End Video` _widget)
          (`Widget.SetVisibility` _widget "Hidden"))))))

(event `/Game/Blueprints/BPI_Queue.Action`
  (bind _fadein (`self.FadeIn`))
  (bind _returnvalue (`|CreateWidget` "/Game/TempDirectory/WBP_Screen.WBP_Screen_C" (`GameplayStatics.GetPlayerController` 0)))
  (`UserWidget.AddToViewport` _returnvalue 0)
  (set `self.Widget` _returnvalue)
  (`TimelineComponent.SetTimelineLength` _fadein (`self.FadeInTime`))
  (`/Game/TempDirectory/WBP_Screen.Play Video` (`self.Widget`))
  (`MediaPlayer.Play` (`self.Media Player`))
  (`Timeline|FadeIn`
    (:`Update`
      (`KismetMaterialLibrary.SetScalarParameterValue` "/Game/TempDirectory/MTPC_Media.MTPC_Media" "Opacity" (`CurveFloat.GetFloatValue` (`self.FadeCurve`) (/ (`TimelineComponent.GetPlaybackPosition` _fadein) (`TimelineComponent.GetTimelineLength` _fadein)))))))

(fn `UserConstructionScript`
  (`parent.UserConstructionScript`))