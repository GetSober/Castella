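; BP_ProbMover moves a target prop along a spline over a set Time, triggered by Action or optionally at BeginPlay.
; A timeline, remapped through MovementCurve, drives location and optional rotation while the prop uses a custom collision channel.
; On finish it notifies its listener, then destroys the prop or restores WorldDynamic, optionally applying last-frame velocity as an impulse.
; Construction sets timeline length and can snap the prop to the spline start.
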(event `self.ReceiveBeginPlay`
  (if (`self.IsBeginplayed`)
    (`self.MoveTarget`)))

(event `MoveTarget`
  (bind _returnvalue (`GameplayStatics.GetWorldDeltaSeconds`))
  (bind _targetprob (`self.TargetProb`))
  (bind _spline (`self.Spline`))
  (bind _time (`self.Time`))
  (bind _movementcurve (`self.MovementCurve`))
  (bind _returnvalue_2 (`SplineComponent.GetSplineLength` _spline))
  (bind _mesh (`/Game/Blueprints/BP_MoveProb.Mesh` (`self.TargetProb`)))
  (`/Game/Blueprints/BP_MoveProb.Impulse To Prob` _targetprob 1.0)
  (`PrimitiveComponent.SetCollisionObjectType` (`/Game/Blueprints/BP_MoveProb.Mesh` _targetprob) "ECC_GameTraceChannel1")
  (`Timeline|타임라인`
    (:`Update`
      (`self.UpdateTimeLine`))
    (:`Finished`
      (`self.OnTimeLineFinished`)
      (if (`self.IsRemove`)
        (`self.K2_DestroyActor` (`self.TargetProb`))
        (else
          (`PrimitiveComponent.SetCollisionObjectType` _mesh "ECC_WorldDynamic")
          (if (`self.IsKeepMove`)
            (`PrimitiveComponent.AddImpulse` _mesh (* (- (`SplineComponent.GetLocationAtDistanceAlongSpline` _spline _returnvalue_2 "World") (`SplineComponent.GetLocationAtDistanceAlongSpline` _spline (`KismetMathLibrary.Lerp` 0.0 _returnvalue_2 (`CurveFloat.GetFloatValue` _movementcurve (* (`.MaxTime` (`CurveBase.GetTimeRange` _movementcurve)) (/ (- _time _returnvalue) _time)))) "World")) (/ 1.0 _returnvalue)) "None" true)))))))

(event `/Game/Blueprints/BPI_Queue.Action`
  (`parent.Action`)
  (`self.MoveTarget`))

(event `/Game/Blueprints/BPI_Queue.RegistActionEndNotify`
  (params (Listener :type "/Game/Blueprints/BPI_ActionEndListener Interface"))
  (set `self.Listener` Listener))

(fn `GetSplineDistance`
  (params (Spline :type "SplineComponent Object Reference"))
  (returns (`Spline Distance By Curve` :type "Float (double-precision)"))
  (bind `_타임라인` (`self.타임라인`))
  (bind _movementcurve (`self.MovementCurve`))
  (return (`KismetMathLibrary.Lerp` 0.0 (`SplineComponent.GetSplineLength` Spline) (`CurveFloat.GetFloatValue` _movementcurve (* (`.MaxTime` (`CurveBase.GetTimeRange` _movementcurve)) (/ (`TimelineComponent.GetPlaybackPosition` `_타임라인`) (`TimelineComponent.GetTimelineLength` `_타임라인`)))))))

(fn `OnTimeLineFinished`
  (`/Game/Blueprints/BPI_ActionEndListener.NotifyActionEnd` (`self.Listener`) "None"))

(fn `UpdateTimeLine`
  (bind _spline (`self.Spline`))
  (bind _spline_2 (`self.Spline`))
  (bind _spline_distance_by_curve (`self.GetSplineDistance` _spline))
  (`SceneComponent.K2_SetWorldLocation` (`/Game/Blueprints/BP_MoveProb.Mesh` (`self.TargetProb`)) (`SplineComponent.GetLocationAtDistanceAlongSpline` _spline _spline_distance_by_curve "World") false false)
  (if (`self.IsSplineAttachedRotation`)
    (bind _spline_distance_by_curve_2 (`self.GetSplineDistance` _spline_2))
    (bind (_returnvalue_roll _returnvalue_pitch _returnvalue_yaw) (`KismetMathLibrary.BreakRotator` (`SplineComponent.GetRotationAtDistanceAlongSpline` _spline_2 _spline_distance_by_curve_2 "Local")))
    (`SceneComponent.K2_SetRelativeRotation` (`/Game/Blueprints/BP_MoveProb.Mesh` (`self.TargetProb`)) (`KismetMathLibrary.MakeRotator` _returnvalue_roll _returnvalue_pitch _returnvalue_yaw) false false)))

(fn `UserConstructionScript`
  (bind _targetprob (`self.TargetProb`))
  (`TimelineComponent.SetTimelineLength` (`self.타임라인`) (`self.Time`))
  (`/Engine/EditorBlueprintResources/StandardMacros.IsValid` _targetprob
    (:`Is Valid`
      (if (`self.IsTargetAttached`)
        (`SceneComponent.K2_SetWorldLocation` (`/Game/Blueprints/BP_MoveProb.Mesh` _targetprob) (`SplineComponent.GetLocationAtSplinePoint` (`self.Spline`) 0 "World") false false)))))