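; BP_Chromakey plays a media source on demand, with an optional fade-in, for a target prop using a media material.
; BeginPlay sets that material on the prop's mesh and separately creates a dynamic instance, without assigning it to the mesh.
; Action starts playback and, if fading, runs a timeline driving the instance's Alpha.
; The construction script sets timeline length to FadeInTime; the fade curve is rescaled to that duration and its value range.
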(event `self.ReceiveBeginPlay`
  (bind _mediamaterial (`self.MediaMaterial`))
  (`PrimitiveComponent.SetMaterial` (`/Game/Blueprints/Queues/BP_MoveProb.Mesh` (`self.TargetProb`)) 0 _mediamaterial)
  (bind _returnvalue (`KismetMaterialLibrary.CreateDynamicMaterialInstance` _mediamaterial))
  (set `self.TargetMeshMaterial` _returnvalue))

(event `/Game/Blueprints/BPI_Queue.Action`
  (bind _mediasource (`self.MediaSource`))
  (bind _fadeincurve (`self.FadeInCurve`))
  (bind (_minvalue _maxvalue) (`CurveBase.GetValueRange` (`self.FadeInCurve`)))
  (bind (_mintime _maxtime) (`CurveBase.GetTimeRange` _fadeincurve))
  (`MediaPlayer.OpenSource` _mediasource (`self.MediaPlayer`))
  (`MediaPlayer.Play` _mediasource)
  (if (`self.IsFadeIn`)
    (`Timeline|타임라인`
      (:`Update`
        (`MaterialInstanceDynamic.SetScalarParameterValue` (`self.TargetMeshMaterial`) "Alpha" (* (`CurveFloat.GetFloatValue` _fadeincurve (* (/ (- _maxtime _mintime) (`self.FadeInTime`)) (`TimelineComponent.GetPlaybackPosition` (`self.타임라인`)))) (/ 1.0 (- _maxvalue _minvalue)))))
      (:`Finished`
        (`MaterialInstanceDynamic.SetScalarParameterValue` (`self.TargetMeshMaterial`) "Alpha" 1.0)))))

(fn `UserConstructionScript`
  (`TimelineComponent.SetTimelineLength` (`self.타임라인`) (`self.FadeInTime`)))