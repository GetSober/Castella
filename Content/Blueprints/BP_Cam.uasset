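; BP_Cam is a camera Blueprint that aligns four child components, Left, Right, Top and Bottom, to angles derived from the camera's field of view.
; On BeginPlay it reads the camera view once, then yaws Left and Right in opposite directions by half the FOV.
; Top and Bottom pitch oppositely by half the arctangent of aspect ratio multiplied by the tangent of half the FOV.
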(event `self.ReceiveBeginPlay`
  (bind _desiredview (`CameraComponent.GetCameraView` (`self.Camera`) 0.0))
  (bind _returnvalue (* (`.FOV` (break `MinimalViewInfo` _desiredview)) -0.5))
  (`SceneComponent.K2_AddRelativeRotation` (`self.Left`) (`KismetMathLibrary.MakeRotator` 0.0 0.0 _returnvalue) false false)
  (`SceneComponent.K2_AddRelativeRotation` (`self.Right`) (`KismetMathLibrary.MakeRotator` 0.0 0.0 (* _returnvalue -1.0)) false false)
  (bind _returnvalue_2 (`KismetMathLibrary.DegAtan` (* (`.AspectRatio` (break `MinimalViewInfo` _desiredview)) (`KismetMathLibrary.DegTan` (* (`.FOV` (break `MinimalViewInfo` _desiredview)) 0.5)))))
  (`SceneComponent.K2_AddRelativeRotation` (`self.Bottom`) (`KismetMathLibrary.MakeRotator` 0.0 (* _returnvalue_2 -0.5)) false false)
  (`SceneComponent.K2_AddRelativeRotation` (`self.Top`) (`KismetMathLibrary.MakeRotator` 0.0 (* _returnvalue_2 0.5)) false false))

(fn `UserConstructionScript`)