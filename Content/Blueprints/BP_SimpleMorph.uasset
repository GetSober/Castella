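; BP_SimpleMorph is an actor that drives a timed morph effect between a skeletal mesh and a Niagara particle system.
; SetNiagaraComponent binds the mesh as the system's target and registers the actor as a particle-data callback, which prints the first particle's position.
; BeginMorph starts feeding the mesh's displacement to Niagara every tick.
; After a delay, a timeline writes normalized progress to the MPC_Morph parameter collection.
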(event `self.ReceiveTick`
  (params (DeltaSeconds :type "Float (single-precision)"))
  (`parent.ReceiveTick` DeltaSeconds)
  (if (`self.bIsMorphing`)
    (`NiagaraComponent.SetVariableVec3` (`self.Niagara`) "User.TargetDeltaPosition" (- (`SceneComponent.K2_GetComponentLocation` (`self.SkeletalMesh`)) (`self.StartPosition`)))))

(event `/Game/Backup/BPI_Morph.BeginMorph`
  (`KismetSystemLibrary.K2_SetTimerDelegate` (delegate `StartMorph`) (`self.MorphingStartDelay`))
  (`TimelineComponent.SetTimelineLength` (`self.MorphingTimeLine`) (`self.MorphingTime`))
  (set `self.StartPosition` (`SceneComponent.K2_GetComponentLocation` (`self.SkeletalMesh`)))
  (set `self.bIsMorphing` true))

(event `StartMorph`
  (bind _morphingtimeline (`self.MorphingTimeLine`))
  (`Timeline|MorphingTimeLine`
    (:`Update`
      (`KismetMaterialLibrary.SetScalarParameterValue` "/Game/Backup/MPC_Morph.MPC_Morph" "Amount1" (/ (`TimelineComponent.GetPlaybackPosition` _morphingtimeline) (`TimelineComponent.GetTimelineLength` _morphingtimeline))))))

(event `/Game/Backup/BPI_Morph.SetNiagaraComponent`
  (params (Niagara :type "NiagaraComponent Object Reference"))
  (bind _output_get (set `self.Niagara` Niagara))
  (`NiagaraFunctionLibrary.OverrideSystemUserVariableSkeletalMeshComponent` _output_get "User.SM_Target" (`self.SkeletalMesh`))
  (`NiagaraComponent.SetVariableObject` _output_get "User.Callback" self))

(event `self.ReceiveParticleData`
  (params (Data :type "Array of BasicParticleData Structure (by ref)") (NiagaraSystem :type "NiagaraSystem Object Reference") (SimulationPositionOffset :type "Vector Structure (by ref)"))
  (bind _output_position (break `BasicParticleData` (`|GetArrayItem` Data)))
  (`KismetSystemLibrary.PrintString` (`KismetStringLibrary.Conv_VectorToString` _output_position)))

(fn `UserConstructionScript`
  (`parent.UserConstructionScript`))