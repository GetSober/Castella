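; Actor that plays a morph-out effect on a skeletal mesh by sliding a box-shaped material mask across it, then hiding itself.
; BeginMorph builds a dynamic material sized from mesh bounds, waits on a timer, then a timeline lerps the mask from MaskPosition to MaskDestination.
; A linked Niagara system receives the mesh as source, plus mask endpoints and rotation.
; Construction script positions visualizers for both mask endpoints.
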(event `self.ReceiveBeginPlay`
  (`self.InitMaskAnim` 5.0 :!label _label))

(event `Init`
  (goto _label))

(event `BeginMaskAnim`
  (params (MaskDelay :type "Float (single-precision)")))

(event `/Game/Blueprints/BPI_Morph.BeginMorph`
  (`self.InitMaskAnim` (`self.MaskAnimTime`))
  (`TimelineComponent.SetTimelineLength` (`self.타임라인`) (`self.MaskAnimTime`))
  (`KismetSystemLibrary.K2_SetTimerDelegate` (delegate `DelayStart`) (`self.MaskAnimDelay`)))

(event `/Game/Blueprints/BPI_Queue.Action`)

(event `DelayStart`
  (`Timeline|타임라인`
    (:`Update`
      (`self.UpdateMask`))
    (:`Finished`
      (`self.SetActorHiddenInGame` true))))

(event `/Game/Blueprints/BPI_Morph.SetNiagaraComponent`
  (params (Niagara :type "NiagaraComponent Object Reference"))
  (bind _output_get (set `self.NiagaraComponent` Niagara))
  (`NiagaraFunctionLibrary.OverrideSystemUserVariableSkeletalMeshComponent` _output_get "User.SM_Source" (`self.MorphingTarget`)))

(fn `InitMaskAnim`
  (params (MaskAnimTime :type "Float (double-precision)"))
  (locals (NewLocalVar :type "Float (double-precision)"))
  (`self.InitMaskAnim_` MaskAnimTime (`self.MaskPosition`) (* (`.BoxExtent` (`KismetMathLibrary.BreakBoxSphereBounds` (`SkeletalMesh.GetBounds` (`SkeletalMeshComponent.GetSkeletalMeshAsset` (`self.MorphingTarget`))))) (2.0 2.0 2.0))))

(fn `InitMaskAnim_`
  (params (MaskAnimTime :type "Float (double-precision)") (MaskPosition :type "Vector Structure") (MaskBoundSize :type "Vector Structure"))
  (bind _morphingtarget (`self.MorphingTarget`))
  (set `self.MaskAnimTime` MaskAnimTime)
  (bind _returnvalue (`PrimitiveComponent.CreateDynamicMaterialInstance` _morphingtarget 0 (`self.Material`) "None"))
  (bind _output_get (set `self.DynamicMaterial` _returnvalue))
  ;[1 1 1] Set Material Params
  (`MaterialInstanceDynamic.SetVectorParameterValue` _output_get "MaskBoxPosition" (`KismetMathLibrary.Conv_VectorToLinearColor` MaskPosition))
  (`MaterialInstanceDynamic.SetVectorParameterValue` _output_get "BoxBoundSize" (`KismetMathLibrary.Conv_VectorToLinearColor` MaskBoundSize))
  (`PrimitiveComponent.SetMaterial` _morphingtarget 0 (`self.DynamicMaterial`))
  (set `self.IsInited` true))

(fn `InitNiagara`
  (params (Niagara :type "NiagaraComponent Object Reference"))
  (bind (_returnvalue_roll _returnvalue_pitch _returnvalue_yaw) (`KismetMathLibrary.BreakRotator` (`SceneComponent.K2_GetComponentRotation` (`self.MorphingTarget`))))
  (`NiagaraComponent.SetVariableVec3` Niagara "User.SourceRegionMaskStartPos" (+ (`SceneComponent.K2_GetComponentLocation` (`self.MorphingTarget`)) (`KismetMathLibrary.Matrix_TransformVector` (`KismetMathLibrary.Conv_TransformToMatrix` (`SceneComponent.K2_GetComponentToWorld` (`self.MorphingTarget`))) (`self.MaskPosition`))))
  (`NiagaraComponent.SetVariableVec3` Niagara "User.SourceRegionMaskRotation" (`KismetMathLibrary.MakeVector` _returnvalue_roll _returnvalue_pitch _returnvalue_yaw))
  (`NiagaraComponent.SetVariableVec3` (`self.NiagaraComponent`) "User.SourceRegionMaskDestPos" (+ (`SceneComponent.K2_GetComponentLocation` (`self.MorphingTarget`)) (`KismetMathLibrary.Matrix_TransformVector` (`KismetMathLibrary.Conv_TransformToMatrix` (`SceneComponent.K2_GetComponentToWorld` (`self.MorphingTarget`))) (`self.MaskDestination`))))
  (`NiagaraComponent.SetVariableVec3` Niagara "User.SourceRegionMaskOffset" (0.0 0.0 0.0)))

(fn `UpdateMask`
  (bind `_타임라인` (`self.타임라인`))
  (`MaterialInstanceDynamic.SetVectorParameterValue` (`self.DynamicMaterial`) "MaskBoxPosition" (`KismetMathLibrary.Conv_VectorToLinearColor` (`KismetMathLibrary.VLerp` (`self.MaskPosition`) (`self.MaskDestination`) (/ (`TimelineComponent.GetPlaybackPosition` `_타임라인`) (`TimelineComponent.GetTimelineLength` `_타임라인`))))))

(fn `UpdateNiagaraVariables`
  (bind (_returnvalue_origin _returnvalue_boxextent) (`KismetMathLibrary.BreakBoxSphereBounds` (`SkeletalMesh.GetBounds` (`SkeletalMeshComponent.GetSkeletalMeshAsset` (`self.MorphingTarget`)))))
  (`BoxComponent.SetBoxExtent` (`self.MaskPositionVisualizer`) _returnvalue_boxextent false)
  (`BoxComponent.SetBoxExtent` (`self.MaskDestinationVisualizer`) _returnvalue_boxextent false)
  (`self.InitMaskAnim_` 0.0 (`self.MaskPosition`) (* _returnvalue_boxextent (2.0 2.0 2.0)))
  (`NiagaraComponent.SetVariableVec3` (`self.NiagaraComponent`) "User.SourceRegionMaskBoxExtent" (* (* _returnvalue_boxextent (`SceneComponent.RelativeScale3D` (`self.RootComponent`))) (3.5 3.5 3.5)))
  (`self.NiagaraComponent`
    (:`then`
      _)
    (:`else`
      ;[1 1 1] Niagara Init Update
      (bind _output_get (set `self.NiagaraComponent` (`self.GetComponentByClass` (`self.NiagaraActor`) "/Script/Niagara.NiagaraComponent")))))
  (`self.InitNiagara` _output_get))

(fn `UserConstructionScript`
  ;[1 1 1] Material Mask Update
  (`SceneComponent.K2_SetRelativeLocation` (`self.MaskPositionVisualizer`) (`self.MaskPosition`) false false)
  (`SceneComponent.K2_SetRelativeLocation` (`self.MaskDestinationVisualizer`) (`self.MaskDestination`) false false)
  (`self.NiagaraComponent`
    (:`then`
      _)
    (:`else`
      ;[1 1 1] Niagara Init Update
      (bind _output_get (set `self.NiagaraComponent` (`self.GetComponentByClass` (`self.NiagaraActor`) "/Script/Niagara.NiagaraComponent")))))
  (`self.InitNiagara` _output_get))