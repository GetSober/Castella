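; Queue manager that steps through an ordered list of BPI_Queue actors, firing the next one's Action on each Q press.
; UpdateQueueList prunes invalid entries, adds new interface implementers found in the level, refreshes names, registers itself for end notifications and runs a swap sort by Number.
; NotifyActionEnd only sets a flag, as the auto-advance logic reading it is disconnected.
; Nothing in this Blueprint calls UpdateQueueList.
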(event `self.ReceiveBeginPlay`
  (`self.EnableInput` (`GameplayStatics.GetPlayerController` 0)))

(event `Key|Q`
  (params (Key :type "Key Structure"))
  (bind _queuelist (`self.QueueList`))
  (bind _curqueuecount (`self.CurQueueCount`))
  (bind _output_queueobj (break `/Game/Blueprints/Queue` (`|GetArrayItem` _queuelist _curqueuecount)))
  (:`Pressed`
    (if (not (>= (`self.CurQueueCount`) (`KismetArrayLibrary.Array_Length` _queuelist)))
      (`/Game/Blueprints/BPI_Queue.Action` _output_queueobj)
      (set `self.CurQueueCount` (+ _curqueuecount 1)))))

(event `Key|Tilde`
  (params (Key :type "Key Structure")))

(event `/Game/Blueprints/BPI_ActionEndListener.NotifyActionEnd`
  (params (ActionName :type Name))
  (set `self.IsActionEnd` true))

(fn `Update Queue List`
  (locals (Queues :type "Array of Actor Object Reference"))
  (bind _queuelist (`self.QueueList`))
  (bind _queuelist_2 (`self.QueueList`))
  (bind _queuelist_3 (`self.QueueList`))
  (`|ExecutionSequence`
    (:`then_0`
      ;[1 1 1] remove deleted queue
      (for (_array_element _array_index) _queuelist
        (`/Engine/EditorBlueprintResources/StandardMacros.IsValid` (`KismetSystemLibrary.Conv_InterfaceToObject` (break `/Game/Blueprints/Queue` _array_element))
          (:`Is Not Valid`
            (`KismetArrayLibrary.Array_Remove` _queuelist _array_index)))))
    (:`then_1`
      (bind _outactors (`GameplayStatics.GetAllActorsWithInterface` "/Game/Blueprints/BPI_Queue.BPI_Queue_C"))
      (bind _output_get (set `local.Queues` _outactors))
      ;[1 1 1] Find New Queue
      (for _array_element_2 (`self.QueueList`)
        (bind _name (`/Game/Blueprints/BPI_Queue.GetName` (break `/Game/Blueprints/Queue` _array_element_2)))
        (for _array_element_3 _output_get
          (bind _asbpi_queue (cast `/Game/Blueprints/BPI_Queue` _array_element_3))
          (bind _name_2 (`/Game/Blueprints/BPI_Queue.GetName` _asbpi_queue))
          (if (== _name_2 _name)
            (`KismetArrayLibrary.Array_RemoveItem` _output_get _array_element_3))))
      ;[1 1 1] Add New Queue
      (for _array_element_4 _output_get
        (bind _asbpi_queue_2 (cast `/Game/Blueprints/BPI_Queue` _array_element_4))
        (bind _name_3 (`/Game/Blueprints/BPI_Queue.GetName` _asbpi_queue_2))
        (`KismetArrayLibrary.Array_Add` (`self.QueueList`) (make `/Game/Blueprints/Queue` _asbpi_queue_2 111 _name_3)))
      ;[1 1 1] Update Name
      (for _index (range (`KismetArrayLibrary.Array_Length` _queuelist_2))
        (bind _output (`|GetArrayItem` _queuelist_2 _index))
        (bind (_queueobj _number) (break `/Game/Blueprints/Queue` _output))
        (bind _name_4 (`/Game/Blueprints/BPI_Queue.GetName` _queueobj))
        (`|VariableSetRef` _output (make `/Game/Blueprints/Queue` _queueobj _number _name_4))
        (`/Game/Blueprints/BPI_Queue.RegistActionEndNotify` _queueobj self)))
    (:`then_2`
      ;[1 1 1] Sort ( < )
      (for (_array_element_5 _array_index_2) _queuelist_3
        (for _index_2 (range _array_index_2 (+ (`KismetArrayLibrary.Array_Length` _queuelist_3) 1))
          (bind (_output_queueobj _output_number) (break `/Game/Blueprints/Queue` (`|GetArrayItem` _queuelist_3 _index_2)))
          (if (< _output_number (`.Number_5_B7F3C9784056C8BCEF84D79DEBDF6CB1` (break `/Game/Blueprints/Queue` _array_element_5)))
            (`KismetArrayLibrary.Array_Swap` _queuelist_3 _index_2 _array_index_2)))))))

(fn `UserConstructionScript`
  (locals (TempQueueList :type "Array of Actor Object Reference") (IsContained :type Boolean))
  (`|ExecutionSequence`))