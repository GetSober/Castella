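; BP_MoveProb is a physics object that gets pushed into a drifting, spinning motion by a one-time impulse.
; ImpulseToProb applies mass-independent linear and angular impulses to its mesh from direction, speed and a scale, firing on BeginPlay when IsAutoEnable is set.
; The construction script randomizes move and rotation directions when their flags are set, then clears the flags so they act as one-shot re-roll toggles.
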(event `self.ReceiveBeginPlay`
  (if (`self.IsAutoEnable`)
    (`self.Impulse To Prob` 1.0)))

(event `self.ReceiveTick`
  (params (DeltaSeconds :type "Float (single-precision)")))

(fn `Impulse To Prob`
  (params (scale :type "Float (double-precision)" :default 1.0))
  (bind _mesh (`self.Mesh`))
  (`PrimitiveComponent.AddImpulse` _mesh (* (`self.MoveDirection`) (* (`self.MoveSpeed`) scale)) "None" true)
  (`PrimitiveComponent.AddAngularImpulseInDegrees` _mesh (* (`self.RotateDirection`) (* (`self.RotateSpeed`) scale)) "None" true))

(fn `UserConstructionScript`
  (if (`self.SetRandomRotDir`)
    (set `self.RotateDirection` (`KismetMathLibrary.RandomUnitVector`))
    (set `self.SetRandomRotDir` false))
  (if (`self.SetRandomMoveDir`)
    (set `self.MoveDirection` (`KismetMathLibrary.RandomUnitVector`))
    (set `self.SetRandomMoveDir` false)))