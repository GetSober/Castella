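; BP_ProbMover_FixedDestination is a child prop mover that re-anchors its movement spline to the target prob's mesh whenever MoveTarget runs.
; It sets the spline's first point to the mesh's world location, then defers to the parent to perform the move.
; With OnlyUseZ, the last point takes the mesh's X and Y and DestinationPoint's Z.
; Otherwise, the last point also takes the mesh's location.
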(event `self.ReceiveBeginPlay`
  (`parent.ReceiveBeginPlay`))

(event `self.MoveTarget`
  (bind _spline (`self.Spline`))
  (bind (_returnvalue_x _returnvalue_y _returnvalue_z) (`KismetMathLibrary.BreakVector` (`SceneComponent.K2_GetComponentLocation` (`self.DestinationPoint`))))
  (bind _mesh (`/Game/Blueprints/BP_MoveProb.Mesh` (`self.TargetProb`)))
  (bind _returnvalue (`SceneComponent.K2_GetComponentLocation` _mesh))
  (bind (_returnvalue_x_2 _returnvalue_y_2) (`KismetMathLibrary.BreakVector` (`SceneComponent.K2_GetComponentLocation` _mesh)))
  (bind _returnvalue_2 (- (`SplineComponent.GetNumberOfSplinePoints` _spline) 1))
  (if (`self.OnlyUseZ`)
    (`SplineComponent.SetLocationAtSplinePoint` _spline _returnvalue_2 (`KismetMathLibrary.MakeVector` _returnvalue_x_2 _returnvalue_y_2 _returnvalue_z) "World" true)
    (else
      (`SplineComponent.SetLocationAtSplinePoint` _spline _returnvalue_2 _returnvalue "World" true)))
  (`SplineComponent.SetLocationAtSplinePoint` _spline 0 _returnvalue "World" true)
  (`parent.MoveTarget`))

(fn `UpdateTimeLine`
  (`parent.UpdateTimeLine`))

(fn `UserConstructionScript`)