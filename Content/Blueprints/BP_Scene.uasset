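; BP_Scene is a Blueprint that switches between two groups of scene actors.
; When an actor stops overlapping Trigger, ChangeScene activates SceneActors2 and closes SceneActors1; the reverse switch to scene 1 is unconnected.
; ActivateScene and CloseScene toggle each actor's visibility, collision and root component visibility without propagating to children.
; Both functions disable actor tick, so activated actors do not resume ticking.
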(event `self.Trigger.OnActorBeginOverlap`
  (params (OverlappedActor :type "Actor Object Reference") (OtherActor :type "Actor Object Reference")))

(event `self.Trigger.OnActorEndOverlap`
  (params (OverlappedActor :type "Actor Object Reference") (OtherActor :type "Actor Object Reference"))
  (set `self.SceneNum` 2)
  (`self.ChangeScene`))

(fn `ActivateScene`
  (params (Array :type "Array of Actor Object Reference"))
  (for _array_element Array
    (`self.SetActorTickEnabled` _array_element false)
    (`self.SetActorHiddenInGame` _array_element false)
    (`self.SetActorEnableCollision` _array_element true)
    (`SceneComponent.SetVisibility` (`Actor.RootComponent` _array_element) true false)))

(fn `ChangeScene`
  (switch `int` (`self.SceneNum`)
    (:`1`
      (`self.ActivateScene` (`self.Scene Actors_1`))
      (`self.CloseScene` (`self.Scene Actors_2`)))
    (:`2`
      (`self.ActivateScene` (`self.Scene Actors_2`))
      (`self.CloseScene` (`self.Scene Actors_1`)))))

(fn `CloseScene`
  (params (Actors :type "Array of Actor Object Reference"))
  (for _array_element Actors
    (`self.SetActorTickEnabled` _array_element false)
    (`self.SetActorHiddenInGame` _array_element true)
    (`self.SetActorEnableCollision` _array_element false)
    (`SceneComponent.SetVisibility` (`Actor.RootComponent` _array_element) false false)))

(fn `UserConstructionScript`)