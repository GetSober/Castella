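; Spawner actor that, once its Action event is called, spawns a configurable class at random intervals until a count limit stops it.
; Tick times each spawn, randomizing location within a scale-sized box, plus rotation and scale, then optionally enables mesh physics and gravity.
; It exposes queue hooks for name and listener registration, but never notifies the stored QueueManager.
; Red debug boxes preview the area at twice the actual spawn extents.
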(event `self.ReceiveTick`
  (params (DeltaSeconds :type "Float (single-precision)"))
  (bind (_returnvalue_x _returnvalue_y _returnvalue_z) (`KismetMathLibrary.BreakVector` (`self.GetActorScale3D`)))
  (bind (_randomrotationmin_roll _randomrotationmin_pitch _randomrotationmin_yaw) (`KismetMathLibrary.BreakRotator` (`self.RandomRotationMin`)))
  (bind (_randomrotationmax_roll _randomrotationmax_pitch _randomrotationmax_yaw) (`KismetMathLibrary.BreakRotator` (`self.RandomRotationMax`)))
  (bind (_randomscalemax_x _randomscalemax_y _randomscalemax_z) (`KismetMathLibrary.BreakVector` (`self.RandomScaleMax`)))
  (bind (_randomscalemin_x _randomscalemin_y _randomscalemin_z) (`KismetMathLibrary.BreakVector` (`self.RandomScaleMin`)))
  (bind _isphysicon (`self.IsPhysicOn`))
  (bind _returnvalue (`KismetMathLibrary.RandomFloatInRange` (`self.SpawnDelayRangeMin`) (`self.SpawnDelayRangeMax`)))
  (if (`self.IsActionCalled`)
    (bind _output_get (set `self.ElapsedTime` (+ (`self.ElapsedTime`) DeltaSeconds)))
    (if (>= _output_get _returnvalue)
      (set `self.ElapsedTime` (- _output_get _returnvalue))
      (bind _result (`/Engine/EditorBlueprintResources/StandardMacros.IncrementInt` (`self.SpawnCounter`))
        (:`  `
          (set `self.IsActionCalled` (< _result (`self.SpawnCount`)))
          (bind _returnvalue_2 (`|SpawnActorFromClass` (`self.SpawnSource`) (`KismetMathLibrary.MakeTransform` (`KismetMathLibrary.RandomPointInBoundingBox` (`self.K2_GetActorLocation`) (`KismetMathLibrary.MakeVector` (* _returnvalue_x 0.5) (* _returnvalue_y 0.5) (* _returnvalue_z 0.5))) (`KismetMathLibrary.MakeRotator` (`KismetMathLibrary.RandomFloatInRange` _randomrotationmin_roll _randomrotationmax_roll) (`KismetMathLibrary.RandomFloatInRange` _randomrotationmin_pitch _randomrotationmax_pitch) (`KismetMathLibrary.RandomFloatInRange` _randomrotationmin_yaw _randomrotationmax_yaw)) (`KismetMathLibrary.MakeVector` (`KismetMathLibrary.RandomFloatInRange` _randomscalemin_x _randomscalemax_x) (`KismetMathLibrary.RandomFloatInRange` _randomscalemin_y _randomscalemax_y) (`KismetMathLibrary.RandomFloatInRange` _randomscalemin_z _randomscalemax_z))) "AdjustIfPossibleButDontSpawnIfColliding" "OverrideRootScale" null null))
          (`/Engine/EditorBlueprintResources/StandardMacros.IsValid` _returnvalue_2
            (:`Is Valid`
              (bind _returnvalue_3 (`self.GetComponentByClass` _returnvalue_2 "/Script/Engine.MeshComponent"))
              (`/Engine/EditorBlueprintResources/StandardMacros.IsValid` _returnvalue_3
                (:`Is Valid`
                  (`PrimitiveComponent.SetSimulatePhysics` _returnvalue_3 _isphysicon)
                  (`PrimitiveComponent.SetEnableGravity` _returnvalue_3 _isphysicon))))))))))

(event `/Game/Blueprints/BPI_Queue.RegistActionEndNotify`
  (params (Listener :type "/Game/Blueprints/BPI_ActionEndListener Interface"))
  (set `self.QueueManager` Listener))

(event `/Game/Blueprints/BPI_Queue.Action`
  (set `self.IsActionCalled` true))

(fn `GetName`
  (returns (Name :type Name))
  (return (`self.QueueName`)))

(fn `ShowSpawnBoxFiveSec`
  (`KismetSystemLibrary.DrawDebugBox` (`self.K2_GetActorLocation`) (* (`self.GetActorScale3D`) (1.0 1.0 1.0)) (struct :`R` 1.0 :`A` 1.0) (`self.K2_GetActorRotation`) 5.0 0.5))

(fn `UserConstructionScript`
  (`KismetSystemLibrary.DrawDebugBox` (`self.K2_GetActorLocation`) (* (`self.GetActorScale3D`) (1.0 1.0 1.0)) (struct :`R` 1.0 :`A` 1.0) (`self.K2_GetActorRotation`) 0.0 0.5))