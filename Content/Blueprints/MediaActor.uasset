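; MediaActor is an actor that plays a media source through a media player as soon as the game begins.
; BeginPlay calls a Play function that opens MediaSource on MediaPlayer and starts playback.
; The construction script does the same after validity checks on both assets, so playback also starts when the actor is constructed.
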(event `self.ReceiveBeginPlay`
  (`self.Play`))

(fn `Play`
  (bind _mediaplayer (`self.MediaPlayer`))
  (`MediaPlayer.OpenSource` _mediaplayer (`self.MediaSource`))
  (`MediaPlayer.Play` _mediaplayer))

(fn `UserConstructionScript`
  (bind _mediasource (`self.MediaSource`)
    (:`then`
      (bind _mediaplayer (`self.MediaPlayer`)
        (:`then`
          (`MediaPlayer.OpenSource` _mediaplayer _mediasource)
          (`MediaPlayer.Play` _mediaplayer))
        (:`else`)))
    (:`else`)))