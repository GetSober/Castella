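; BP_Chromakey plays a media video on a target actor's mesh through a dynamic material, as a queued action.
; BeginPlay sets up the material at zero Alpha and opens the source; Action starts playback and optional fade-in.
; Tick starts the optional fade-out near the video's end, and media end notifies QueueManager.
; Both fades drive Alpha from float curves, scaling timeline position to the curve's time range for configurable durations.
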(event `self.ReceiveBeginPlay`
  (bind _mediaplayer (`self.MediaPlayer`))
  (`parent.ReceiveBeginPlay`)
  (bind _returnvalue (`KismetMaterialLibrary.CreateDynamicMaterialInstance` (`self.MediaMaterial`)))
  (bind _output_get (set `self.DynamicMaterial` _returnvalue))
  (`PrimitiveComponent.SetMaterial` (`self.TargetMesh`) 0 _output_get)
  (`MaterialInstanceDynamic.SetTextureParameterValue` _output_get "MediaTexture" (`self.MediaTexture`))
  (`MaterialInstanceDynamic.SetScalarParameterValue` (`self.DynamicMaterial`) "Alpha" 0.0)
  (`TimelineComponent.SetTimelineLength` (`self.FadeInTimeLine`) (`self.FadeInTime`))
  (`TimelineComponent.SetTimelineLength` (`self.FadeOutTimeLine`) (`self.FadeOutTime`))
  ;[1 1 1] Media Player Init
  (`MediaPlayer.OpenSource` _mediaplayer (`self.MediaSource`))
  (add `MediaPlayer.OnEndReached` _mediaplayer (delegate `On Media End`)))

(event `On Media End`
  (`/Game/Blueprints/BPI_ActionEndListener.NotifyActionEnd` (`self.QueueManager`) (`self.QueueName`))
  (`KismetSystemLibrary.PrintString` "End"))

(event `self.ReceiveTick`
  (params (DeltaSeconds :type "Float (single-precision)"))
  (bind (_returnvalue_days _returnvalue_hours _returnvalue_minutes _returnvalue_seconds) (`KismetMathLibrary.BreakTimespan` (`MediaPlayer.GetTime` (`self.MediaPlayer`))))
  (`parent.ReceiveTick` DeltaSeconds)
  (if (and (`self.IsFadeOut`) (<= (- (`self.MediaDuration`) _returnvalue_seconds) (`self.FadeOutTime`)))
    (`Timeline|FadeOutTimeLine`
      (:`Update`
        _)
      (:`Finished`
        _))
    (bind _curvevalue (`self.Curve Float with Time Line` (`self.FadeOutTimeLine`) (`self.FadeOutCurve`) (`self.FadeOutTime`)))
    (`MaterialInstanceDynamic.SetScalarParameterValue` (`self.DynamicMaterial`) "Alpha" (- 1.0 _curvevalue))))

(event `/Game/Blueprints/BPI_Queue.Action`
  (bind _mediaplayer (`self.MediaPlayer`))
  (bind (_returnvalue_days _returnvalue_hours _returnvalue_minutes _returnvalue_seconds) (`KismetMathLibrary.BreakTimespan` (`MediaPlayer.GetDuration` _mediaplayer)))
  (set `self.MediaDuration` (`KismetMathLibrary.Conv_IntToDouble` _returnvalue_seconds))
  (`MediaPlayer.Play` _mediaplayer)
  (if (`self.IsFadeIn`)
    (`Timeline|FadeInTimeLine`
      (:`Update`
        _)
      (:`Finished`
        _))
    (bind _curvevalue (`self.Curve Float with Time Line` (`self.FadeInTimeLine`) (`self.FadeInCurve`) (`self.FadeInTime`)))
    (`MaterialInstanceDynamic.SetScalarParameterValue` (`self.DynamicMaterial`) "Alpha" _curvevalue)))

(fn `Curve Float with Time Line`
  (params (TimeLine :type "TimelineComponent Object Reference") (CurveFloat :type "CurveFloat Object Reference") (TimeLineLength :type "Float (double-precision)"))
  (returns (CurveValue :type "Float (single-precision)"))
  (bind (_mintime _maxtime) (`CurveBase.GetTimeRange` CurveFloat))
  (return (`CurveFloat.GetFloatValue` CurveFloat (* (`TimelineComponent.GetPlaybackPosition` TimeLine) (/ (- _maxtime _mintime) TimeLineLength)))))

(fn `UserConstructionScript`
  (`parent.UserConstructionScript`)
  (bind _targetactor (`self.TargetActor`)
    (:`then`
      (bind _returnvalue (`self.GetComponentByClass` _targetactor "/Script/Engine.MeshComponent"))
      (`/Engine/EditorBlueprintResources/StandardMacros.IsValid` _returnvalue
        (:`Is Valid`
          (set `self.TargetMesh` _returnvalue))))
    (:`else`)))