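; Test actor for a Niagara morphing effect that runs alongside a mask animation on a Source object.
; BeginPlay passes itself, the Arrow's forward vector and the Source's morph-target skeletal mesh to Niagara, and construction also sets the vector.
; StartMorphingEffect feeds ParticleTime to both the particle lerp and the Source's mask animation, then starts both.
; A particle data callback prints each particle's size.
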(event `self.ReceiveBeginPlay`
  (bind _niagara (`self.Niagara`))
  (`NiagaraComponent.SetVariableObject` _niagara "User.Owner" self)
  (`NiagaraComponent.SetVariableVec3` _niagara "User.ForwardVector" (`SceneComponent.GetForwardVector` (`self.Arrow`)))
  (`NiagaraFunctionLibrary.OverrideSystemUserVariableSkeletalMeshComponent` _niagara "SM_Source" (`/Game/Backup/BP_MaskAnimActor.MorphingTarget` (`self.Source`))))

(event `self.ReceiveParticleData`
  (params (Data :type "Array of BasicParticleData Structure (by ref)") (NiagaraSystem :type "NiagaraSystem Object Reference") (SimulationPositionOffset :type "Vector Structure (by ref)"))
  (for _array_element Data
    (`KismetSystemLibrary.PrintString` (`KismetStringLibrary.Conv_DoubleToString` (`.Size` (break `BasicParticleData` _array_element))))))

(event `Start Morphing Effect`
  (bind _niagara (`self.Niagara`))
  (bind _particletime (`self.ParticleTime`))
  (bind _source (`self.Source`))
  (`NiagaraComponent.SetVariableFloat` _niagara "User.LerpTime" _particletime)
  (`/Game/Backup/BP_MaskAnimActor.InitMaskAnim` _source _particletime)
  (`/Game/Backup/BP_MaskAnimActor.BeginMaskAnim` _source)
  (`ActorComponent.Activate` _niagara false))

(fn `UserConstructionScript`
  (`NiagaraComponent.SetVariableVec3` (`self.Niagara`) "User.ForwardVector" (`SceneComponent.GetForwardVector` (`self.Arrow`))))