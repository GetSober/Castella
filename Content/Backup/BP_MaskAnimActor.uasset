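; Actor that animates a box-shaped material mask moving across a skeletal mesh (MorphingTarget) from a start to a destination position.
; Construction and BeginPlay or Init create a dynamic material on slot 0, setting the mask box position and a size taken from the mesh bounds.
; BeginMaskAnim runs a timeline of configurable length, lerping the box position parameter by normalized playback time.
; Two box visualizers preview the start and destination positions.
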(event `self.ReceiveBeginPlay`
  (`self.InitMaskAnim` 5.0 :!label _label))

(event `Init`
  (goto _label))

(event `BeginMaskAnim`
  (if (`self.IsInited`)
    (`TimelineComponent.SetTimelineLength` (`self.타임라인`) (`self.MaskAnimTime`))
    (`Timeline|타임라인`
      (:`Update`
        _)
      (:`Finished`
        _))
    (`self.UpdateMask`)
    (else
      (`KismetSystemLibrary.LogString` (`KismetStringLibrary.Concat_StrStr` (`KismetSystemLibrary.GetClassDisplayName` (`GameplayStatics.GetObjectClass` self)) "not initialized")))))

(fn `InitMaskAnim`
  (params (MaskAnimTime :type "Float (double-precision)"))
  (locals (NewLocalVar :type "Float (double-precision)"))
  (`self.InitMaskAnim_` MaskAnimTime (`self.MaskPosition`) (* (`.BoxExtent` (`KismetMathLibrary.BreakBoxSphereBounds` (`SkeletalMesh.GetBounds` (`SkeletalMeshComponent.GetSkeletalMeshAsset` (`self.MorphingTarget`))))) (2.0 2.0 2.0))))

(fn `InitMaskAnim_`
  (params (MaskAnimTime :type "Float (double-precision)") (MaskPosition :type "Vector Structure") (MaskBoundSize :type "Vector Structure"))
  (bind _morphingtarget (`self.MorphingTarget`))
  (set `self.MaskAnimTime` MaskAnimTime)
  (bind _returnvalue (`PrimitiveComponent.CreateDynamicMaterialInstance` _morphingtarget 0 (`self.Material`) "None"))
  (bind _output_get (set `self.DynamicMaterial` _returnvalue))
  ;[1 1 1] Set Material Params
  (`MaterialInstanceDynamic.SetVectorParameterValue` _output_get "MaskBoxPosition" (`KismetMathLibrary.Conv_VectorToLinearColor` MaskPosition))
  (`MaterialInstanceDynamic.SetVectorParameterValue` _output_get "BoxBoundSize" (`KismetMathLibrary.Conv_VectorToLinearColor` MaskBoundSize))
  (`PrimitiveComponent.SetMaterial` _morphingtarget 0 (`self.DynamicMaterial`))
  (set `self.IsInited` true))

(fn `UpdateMask`
  (bind `_타임라인` (`self.타임라인`))
  (`MaterialInstanceDynamic.SetVectorParameterValue` (`self.DynamicMaterial`) "MaskBoxPosition" (`KismetMathLibrary.Conv_VectorToLinearColor` (`KismetMathLibrary.VLerp` (`self.MaskPosition`) (`self.MaskDestination`) (/ (`TimelineComponent.GetPlaybackPosition` `_타임라인`) (`TimelineComponent.GetTimelineLength` `_타임라인`))))))

(fn `UserConstructionScript`
  (bind (_returnvalue_origin _returnvalue_boxextent) (`KismetMathLibrary.BreakBoxSphereBounds` (`SkeletalMesh.GetBounds` (`SkeletalMeshComponent.GetSkeletalMeshAsset` (`self.MorphingTarget`)))))
  (`SceneComponent.K2_SetRelativeLocation` (`self.MaskPositionVisualizer`) (`self.MaskPosition`) false false)
  (`BoxComponent.SetBoxExtent` (`self.MaskPositionVisualizer`) _returnvalue_boxextent false)
  (`SceneComponent.K2_SetRelativeLocation` (`self.MaskDestinationVisualizer`) (`self.MaskDestination`) false false)
  (`BoxComponent.SetBoxExtent` (`self.MaskDestinationVisualizer`) _returnvalue_boxextent false)
  (`self.InitMaskAnim_` 0.0 (`self.MaskPosition`) (* _returnvalue_boxextent (2.0 2.0 2.0))))