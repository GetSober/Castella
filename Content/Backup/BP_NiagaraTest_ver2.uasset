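; A test actor that starts a Niagara morph effect between a Source and a Target.
; StartMorphingEffect or Action calls ActionAllChain, then hands the Niagara component to Source and begins its morph through BPI_Morph messages.
; If Source and Target both implement the interface, Target receives the same messages and Niagara activates.
; The construction script feeds the Arrow's forward vector into the Niagara ForwardVector user parameter.
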(event `self.ReceiveBeginPlay`)

(event `Start Morphing Effect`
  (bind _target (`self.Target`))
  (bind _source (`self.Source`))
  (`self.ActionAllChain` :!label _label)
  (if (`KismetSystemLibrary.DoesImplementInterface` _source "/Game/Backup/BPI_Morph.BPI_Morph_C")
    (message `/Game/Backup/BPI_Morph.SetNiagaraComponent` _source (`self.Niagara`))
    (message `/Game/Backup/BPI_Morph.BeginMorph` _source)
    (if (`KismetSystemLibrary.DoesImplementInterface` _target "/Game/Backup/BPI_Morph.BPI_Morph_C")
      (message `/Game/Backup/BPI_Morph.SetNiagaraComponent` _target (`self.Niagara`))
      (message `/Game/Backup/BPI_Morph.BeginMorph` _target)
      (`ActorComponent.Activate` (`self.Niagara`) false))))

(event `/Game/Blueprints/BPI_Queue.Action`
  (goto _label))

(fn `UserConstructionScript`
  (`NiagaraComponent.SetVariableVec3` (`self.Niagara`) "User.ForwardVector" (`SceneComponent.GetForwardVector` (`self.Arrow`))))